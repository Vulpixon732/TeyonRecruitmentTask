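; BP_3DPrinter is an interactable, powered printer that spawns a "PrintedKeycard" item pickup.
; Using an AutoHack, Keycard or PrintedKeycard while active starts it, consuming all but the Keycard, and closes a gate against reuse.
; A timeline moves the printer parts, then spawns the pickup at DropPoint and starts blinking "OUT OF INK" text.
; AssignState toggles power, updating text visibility and freezing or resuming a running animation via play rate.
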(event Custom|DebugAnimation
  (bind _inkhorizontal (Variables|Default|GetInkHorizontal))
  (bind _printeranimation (Variables|Default|GetPrinterAnimation))
  (bind _printerinside (Variables|Default|GetPrinterInside))
  (bind _textrender (Variables|Default|GetTextRender))
  (bind _returnvalue (Transformation|GetRelativeTransform _printerinside))
  (bind _returnvalue_2 (Transformation|GetRelativeTransform _inkhorizontal))
  (Components|Timeline|SetPlayRate _printeranimation (Variables|Default|GetAnimationPlayRate))
  (if (not (Components|Activation|IsActive _printeranimation))
    (bind (_direction _printerinside_2 _inkhorizontal_2) (Timeline|PrinterAnimation PlayFromStart)
      (:Update
        (Utilities|FlowControl|Sequence
          (:then_0
            (Transformation|SetRelativeLocation _printerinside (Math|Vector|MakeVector (.x _printerinside_2) (.y (.location _returnvalue)) (.z (.location _returnvalue))) false true))
          (:then_1
            (Transformation|SetRelativeLocation _inkhorizontal (Math|Vector|MakeVector (.x (.location _returnvalue_2)) (.y _inkhorizontal_2) (.z (.location _returnvalue_2))) false true))))
      (:Finished
        (Game|SpawnActorfromClass "/Game/TeyonTask/Blueprints/Items/BP_ItemPickup.BP_ItemPickup_C" (Transformation|GetWorldTransform (Variables|Default|GetDropPoint)) "AdjustIfPossibleButAlwaysSpawn" "MultiplyWithRoot" 0 (Utilities|Struct|MakeS_ItemData "PrintedKeycard" "None" "None") "None" "None" 0)
        (Rendering|Components|TextRender|SetText (Variables|Default|GetTextRender) (Utilities|Text|MakeLiteralText "Out of Ink"))
        (Timeline|TextBlink Play
          (:Trigger
            (Rendering|Components|TextRender|SetText _textrender (Utilities|String|SelectText "OUT OF INK" "NO POWER" (Variables|Default|GetIsActive)))
            (if (Variables|Default|GetIsActive)
              (Rendering|SetVisibility _textrender (not (Variables|/Script/Engine.SceneComponent|GetbVisible _textrender)) false)
              (else
                (Rendering|SetVisibility _textrender true false)))))))))

(event Custom|BeginPrinting
  (bind _inkhorizontal (Variables|Default|GetInkHorizontal))
  (bind _printeranimation (Variables|Default|GetPrinterAnimation))
  (bind _printerinside (Variables|Default|GetPrinterInside))
  (bind _textrender (Variables|Default|GetTextRender))
  (bind _returnvalue (Transformation|GetRelativeTransform _printerinside))
  (bind _returnvalue_2 (Transformation|GetRelativeTransform _inkhorizontal))
  (Components|Timeline|SetPlayRate _printeranimation (Variables|Default|GetAnimationPlayRate))
  (if (not (Components|Activation|IsActive _printeranimation))
    (bind (_direction _printerinside_2 _inkhorizontal_2) (Timeline|PrinterAnimation PlayFromStart)
      (:Update
        (Utilities|FlowControl|Sequence
          (:then_0
            (Transformation|SetRelativeLocation _printerinside (Math|Vector|MakeVector (.x _printerinside_2) (.y (.location _returnvalue)) (.z (.location _returnvalue))) false true))
          (:then_1
            (Transformation|SetRelativeLocation _inkhorizontal (Math|Vector|MakeVector (.x (.location _returnvalue_2)) (.y _inkhorizontal_2) (.z (.location _returnvalue_2))) false true))))
      (:Finished
        (Game|SpawnActorfromClass "/Game/TeyonTask/Blueprints/Items/BP_ItemPickup.BP_ItemPickup_C" (Transformation|GetWorldTransform (Variables|Default|GetDropPoint)) "AdjustIfPossibleButAlwaysSpawn" "MultiplyWithRoot" 0 (Utilities|Struct|MakeS_ItemData "PrintedKeycard" "None" "None") "None" "None" 0)
        (Rendering|Components|TextRender|SetText (Variables|Default|GetTextRender) (Utilities|Text|MakeLiteralText "Out of Ink"))
        (Timeline|TextBlink Play
          (:Trigger
            (Rendering|Components|TextRender|SetText _textrender (Utilities|String|SelectText "OUT OF INK" "NO POWER" (Variables|Default|GetIsActive)))
            (if (Variables|Default|GetIsActive)
              (Rendering|SetVisibility _textrender (not (Variables|/Script/Engine.SceneComponent|GetbVisible _textrender)) false)
              (else
                (Rendering|SetVisibility _textrender true false)))))))))

(event EventBeginPlay)

(event Collision|EventActorBeginOverlap
  (params (OtherActor :type Actor%20Object%20Reference)))

(event EventTick
  (params (DeltaSeconds :type Float%20%28single-precision%29)))

(event EventOnItemInteract
  (params (UsedItem :type Name :default "None") (EventCaller :type Actor%20Object%20Reference))
  (Utilities|FlowControl|Gate false :!label _label
    (:Exit
      (if (Variables|Default|GetIsActive)
        (bind _asbp_teyon_first_person_character (Utilities|Casting|CastToBP_Teyon_FirstPersonCharacter EventCaller))
        (if (or (== UsedItem "AutoHack") (== UsedItem "PrintedKeycard"))
          (Default|DestroyActiveItem (Variables|/Game/TeyonTask/Blueprints/PlayerCharacter/BP_Teyon_FirstPersonCharacter.BP_Teyon_FirstPersonCharacter_C|GetAC_InventoryComponent _asbp_teyon_first_person_character))
          (CallFunction|BeginPrinting :!label _label_2)
          (goto _label Close)
          (elif (== UsedItem "Keycard")
            (goto _label_2)))))))

(event EventAssignState
  (params (IsActive :type Boolean))
  (bind _printeranimation (Variables|Default|GetPrinterAnimation))
  (Variables|Default|SetIsActive IsActive)
  (CallFunction|UpdateVisuals)
  (if (Components|Activation|IsActive _printeranimation)
    (Components|Timeline|SetPlayRate _printeranimation (Math|Float|SelectFloat (Variables|Default|GetAnimationPlayRate) 0.0 (Variables|Default|GetIsActive)))))

(fn ConstructionScript)

(fn UpdateVisuals
  (Rendering|SetVisibility (Variables|Default|GetTextRender) (not (Variables|Default|GetIsActive)) false))