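; BP_Powerbox is an interactible power box that toggles a running state and passes it to a linked TargetActor.
; Interacting flips the state if the box is connected and intact, while a player's Crowbar destroys it, losing durability and forcing it off.
; State changes swap box and light materials, message the target and fire a toggled event.
; The construction script applies the same visuals and target state at construction.
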(event Custom|UpdateState
  (CallFunction|UpdateVisuals)
  (Class|IPowerConnection|AssignState(Message) (Variables|Default|GetTargetActor) (Variables|Default|GetIsRunning))
  (Default|CallEventToggled))

(event EventBeginPlay)

(event Collision|EventActorBeginOverlap
  (params (OtherActor :type Actor%20Object%20Reference)))

(event EventTick
  (params (DeltaSeconds :type Float%20%28single-precision%29)))

(event EventOnItemInteract
  (params (UsedItem :type Name :default "None") (EventCaller :type Actor%20Object%20Reference))
  (bind _asbp_teyon_first_person_character (Utilities|Casting|CastToBP_Teyon_FirstPersonCharacter EventCaller)
    (:then
      (if (and (== UsedItem "Crowbar") (not (Variables|Default|GetIsDestroyed)))
        (Default|ReduceDurability (Variables|/Game/TeyonTask/Blueprints/PlayerCharacter/BP_Teyon_FirstPersonCharacter.BP_Teyon_FirstPersonCharacter_C|GetAC_InventoryComponent _asbp_teyon_first_person_character) 1e+01)
        (CallFunction|ChangeDestroyState true)
        (CallFunction|UpdateState)
        (else
          (if (and (not (Variables|Default|GetIsDestroyed)) (Variables|Default|GetPowerConnected)) :!label _label
            (Variables|Default|SetIsRunning (not (Variables|Default|GetIsRunning)))
            (CallFunction|UpdateState)))))
    (:CastFailed
      (goto _label))))

(fn ConstructionScript
  (bind _targetactor (Variables|Default|GetTargetActor))
  (CallFunction|UpdateVisuals)
  (Utilities|IsValid _targetactor
    (:Is%20Valid
      (Class|IPowerConnection|AssignState(Message) _targetactor (Variables|Default|GetIsRunning)))))

(fn UpdateVisuals
  (bind _isdestroyed (Variables|Default|GetIsDestroyed))
  (Rendering|Material|SetMaterial (Variables|Default|GetLightCube) 0 (select _isdestroyed "/Engine/MapTemplates/Materials/BasicAsset02.BasicAsset02" (select (Variables|Default|GetIsRunning) "/Engine/MapTemplates/Materials/BasicAsset03.BasicAsset03" "/Engine/MapTemplates/Materials/BasicAsset01.BasicAsset01")))
  (Rendering|Material|SetMaterial (Variables|Default|GetCube) 0 (select _isdestroyed "/Engine/BufferVisualization/Anisotropy.Anisotropy" "/Engine/BasicShapes/BasicShapeMaterial.BasicShapeMaterial")))

(fn ChangeDestroyState
  (params (NewState :type Boolean))
  (bind _output_get (Variables|Default|SetIsDestroyed NewState))
  (if (and _output_get (Variables|Default|GetIsRunning))
    (Variables|Default|SetIsRunning false)))

(fn AssignIsRunning
  (params (IsRunning :type Boolean))
  (Variables|Default|SetIsRunning IsRunning)
  (CallFunction|UpdateState))