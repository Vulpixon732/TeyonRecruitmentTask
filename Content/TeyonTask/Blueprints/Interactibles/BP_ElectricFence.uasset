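; BP_ElectricFence is an electric fence actor with an adjustable length and an active or inactive look.
; The construction script uses Distance to place the end piece, centre the middle scene component and stretch the fence along X.
; AssignState sets IsActive and calls UpdateVisual, which also runs on BeginPlay and switches between pulsing and plain hex-tile materials.
; The graphs shown handle only layout and visuals, with no damage or overlap logic.
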(event EventBeginPlay
  (CallFunction|UpdateVisual))

(event Collision|EventActorBeginOverlap
  (params (OtherActor :type Actor%20Object%20Reference)))

(event EventTick
  (params (DeltaSeconds :type Float%20%28single-precision%29)))

(event EventAssignState
  (params (IsActive :type Boolean))
  (Variables|Default|SetIsActive IsActive)
  (CallFunction|UpdateVisual))

(fn ConstructionScript
  (bind _electricfence (Variables|Default|GetElectricFence))
  (bind _relativescale3d (Variables|/Script/Engine.SceneComponent|GetRelativeScale3D _electricfence))
  (Utilities|FlowControl|Sequence
    (:then_0
      (Transformation|SetRelativeLocation (Variables|Default|GetFenceEnd) (Math|Vector|MakeVector (Variables|Default|GetDistance) 0.0 0.0) false false))
    (:then_1
      (Transformation|SetRelativeLocation (Variables|Default|GetFenceMiddleScene) (Math|Vector|MakeVector (/ (Variables|Default|GetDistance) 2.0) 0.0 0.0) false false))
    (:then_2
      (Transformation|SetRelativeScale3D _electricfence (Math|Vector|MakeVector (/ (Variables|Default|GetDistance) 1e+03) (.y _relativescale3d) (.z _relativescale3d))))))

(fn UpdateVisual
  (Rendering|Material|SetMaterial (Variables|Default|GetElectricFence) 0 (select (Variables|Default|GetIsActive) "/Game/StarterContent/Materials/M_Tech_Hex_Tile_Pulse.M_Tech_Hex_Tile_Pulse" "/Game/StarterContent/Materials/M_Tech_Hex_Tile.M_Tech_Hex_Tile")))