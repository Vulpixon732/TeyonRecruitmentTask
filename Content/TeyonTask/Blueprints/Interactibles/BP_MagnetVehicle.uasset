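; BP_MagnetVehicle is an interactable that hands the local player control of a referenced magnet pawn.
; On interact, if it is active and the first-person character belongs to player controller 0, that controller possesses MagnetRef and calls its visibility update.
; AssignState sets the active flag, then UpdateState calls Unpossess on the magnet regardless of the new value.
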(event Custom|UpdateState
  (Default|Unpossess (Variables|Default|GetMagnetRef)))

(event EventBeginPlay)

(event Collision|EventActorBeginOverlap
  (params (OtherActor :type Actor%20Object%20Reference)))

(event EventTick
  (params (DeltaSeconds :type Float%20%28single-precision%29)))

(event EventOnInteract
  (params (PlayerActor :type Actor%20Object%20Reference))
  (bind _magnetref (Variables|Default|GetMagnetRef))
  (bind _asbp_teyon_first_person_character (Utilities|Casting|CastToBP_Teyon_FirstPersonCharacter PlayerActor))
  (if (and (== (Pawn|GetController _asbp_teyon_first_person_character) (Game|GetPlayerController 0)) (Variables|Default|GetIsActive))
    (Utilities|IsValid (Variables|Default|GetMagnetRef)
      (:Is%20Valid
        (Pawn|Possess (Game|GetPlayerController 0) _magnetref)
        (Default|UpdateVisiblity _magnetref)))))

(event EventAssignState
  (params (IsActive :type Boolean))
  (Variables|Default|SetIsActive IsActive)
  (CallFunction|UpdateState))

(fn ConstructionScript)