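; Interactable terminal that the player unlocks, then uses to switch power on its connected power controllers.
; AutoHack, PrintedKeycard or Keycard grants access, consuming all but the Keycard; later interactions toggle power and refresh each controller's connections.
; A Crowbar is consumed to deactivate the terminal and blank its screen, without notifying the controllers.
; The construction script syncs screen material and status texts to the state variables.
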(event EventBeginPlay)

(event Collision|EventActorBeginOverlap
  (params (OtherActor :type Actor%20Object%20Reference)))

(event EventTick
  (params (DeltaSeconds :type Float%20%28single-precision%29)))

(event EventOnItemInteract
  (params (UsedItem :type Name :default "None") (EventCaller :type Actor%20Object%20Reference))
  (if (Variables|Default|GetIsActive)
    (bind _asbp_teyon_first_person_character (Utilities|Casting|CastToBP_Teyon_FirstPersonCharacter EventCaller))
    (if (== UsedItem "Crowbar")
      (Variables|Default|SetPowerState false)
      (Variables|Default|SetIsActive false)
      (CallFunction|UpdateScreenCube)
      (Default|DestroyActiveItem (Variables|/Game/TeyonTask/Blueprints/PlayerCharacter/BP_Teyon_FirstPersonCharacter.BP_Teyon_FirstPersonCharacter_C|GetAC_InventoryComponent _asbp_teyon_first_person_character))
      (elif (not (Variables|Default|GetIsAccessGranted))
        (if (or (== UsedItem "AutoHack") (== UsedItem "PrintedKeycard"))
          (Default|DestroyActiveItem (Variables|/Game/TeyonTask/Blueprints/PlayerCharacter/BP_Teyon_FirstPersonCharacter.BP_Teyon_FirstPersonCharacter_C|GetAC_InventoryComponent _asbp_teyon_first_person_character))
          (Variables|Default|SetIsAccessGranted true :!label _label)
          (CallFunction|UpdateAccessText)
          (elif (== UsedItem "Keycard")
            (goto _label)))
        (else
          (CallFunction|TogglePowerState)
          (CallFunction|UpdatePowerText)
          (CallFunction|ChangeControllerPowerState (Variables|Default|GetPowerState)))))))

(fn ConstructionScript
  (Utilities|FlowControl|Sequence
    (:then_0
      (CallFunction|UpdateScreenCube))
    (:then_1
      (CallFunction|UpdateAccessText))
    (:then_2
      (CallFunction|UpdatePowerText))))

(fn UpdateScreenCube
  (bind _isactive (Variables|Default|GetIsActive))
  (Utilities|FlowControl|Sequence
    (:then_0
      (Rendering|Material|SetMaterial (Variables|Default|GetScreenCube) 0 (select _isactive "/Game/LevelPrototyping/Materials/MI_Solid_Blue.MI_Solid_Blue" "/Game/LevelPrototyping/Materials/M_Solid.M_Solid")))
    (:then_1
      (Rendering|SetVisibility (Variables|Default|GetTextRender) _isactive false))
    (:then_2
      (Rendering|SetVisibility (Variables|Default|GetTextRender1) _isactive false))))

(fn UpdateAccessText
  (Rendering|Components|TextRender|SetText (Variables|Default|GetTextRender) (Utilities|String|SelectText "ACCESS 
GRANTED" "AUTHENTICATION 
REQUIRED" (Variables|Default|GetIsAccessGranted))))

(fn UpdatePowerText
  (bind _textrender1 (Variables|Default|GetTextRender1))
  (bind _powerstate (Variables|Default|GetPowerState))
  (Utilities|FlowControl|Sequence
    (:then_0
      (Rendering|Components|TextRender|SetText _textrender1 (Utilities|String|SelectText "POWER 
ONLINE" "POWER 
OFFLINE" _powerstate)))
    (:then_1
      (Rendering|Components|TextRender|SetTextRenderColor _textrender1 (select _powerstate (Math|Color|MakeColor 41 156 0 255) (Math|Color|MakeColor 0 0 156 255))))))

(fn TogglePowerState
  (Variables|Default|SetPowerState (not (Variables|Default|GetPowerState))))

(fn ChangeControllerPowerState
  (params (NewState :type Boolean))
  (for _array_element (Variables|Default|GetConnectedPowerControllers)
    (Variables|/Game/TeyonTask/Blueprints/Interactibles/BP_PowerController.BP_PowerController_C|SetIsActive _array_element NewState)
    (Default|ChangePowerConnections _array_element)))