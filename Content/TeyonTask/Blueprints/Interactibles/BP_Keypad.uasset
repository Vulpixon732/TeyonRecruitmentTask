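; BP_Keypad is an interactable in-world code keypad that sends an interact message to its target actor when the correct code is entered.
; It binds to the code event of its W_Keypad widget component and toggles Game-and-UI input as its WidgetInteraction hover changes.
; Using an AutoHack item reveals the hidden code and consumes that item.
; The construction script randomizes the interaction's virtual user index.
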(event OnHoveredWidgetChanged(WidgetInteraction)
  (params (WidgetComponent :type Widget%20Component%20Object%20Reference) (PreviousWidgetComponent :type Widget%20Component%20Object%20Reference))
  (bind _returnvalue (Game|GetPlayerController 0))
  (if (Utilities|IsValid WidgetComponent)
    (Input|SetInputModeGameandUI _returnvalue (UserInterface|GetWidget (Variables|Default|GetWidget)) "DoNotLock" true false)
    (else
      (Input|SetInputModeGameOnly _returnvalue false))))

(event Custom|CorrectCodeInserted
  (Class|BPBPIQuestsInteraction|OnInteract(Message) (Variables|Components|GetTargetActor) self))

(event EventBeginPlay
  (bind _asw_keypad (Utilities|Casting|CastToW_Keypad (UserInterface|GetWidget (Variables|Default|GetWidget))))
  (bind _output_get (Variables|Default|Set%20W_KeypadRef _asw_keypad))
  (EventDispatchers|BindEventtoEventCorrectCodeInserted _output_get (delegate Custom|CorrectCodeInserted)))

(event Collision|EventActorBeginOverlap
  (params (OtherActor :type Actor%20Object%20Reference)))

(event EventTick
  (params (DeltaSeconds :type Float%20%28single-precision%29)))

(event EventOnItemInteract
  (params (UsedItem :type Name :default "None") (EventCaller :type Actor%20Object%20Reference))
  (bind __w_keypadref (Variables|Default|Get%20W_KeypadRef))
  (bind _asbp_teyon_first_person_character (Utilities|Casting|CastToBP_Teyon_FirstPersonCharacter EventCaller))
  (if (and (== UsedItem "AutoHack") (not (Widget|IsVisible (Variables|/Game/TeyonTask/Blueprints/Widgets/W_Keypad.W_Keypad_C|GetDebug_Code __w_keypadref))))
    (Default|RevealCode __w_keypadref)
    (Default|DestroyActiveItem (Variables|/Game/TeyonTask/Blueprints/PlayerCharacter/BP_Teyon_FirstPersonCharacter.BP_Teyon_FirstPersonCharacter_C|GetAC_InventoryComponent _asbp_teyon_first_person_character))))

(fn ConstructionScript
  (Variables|/Script/UMG.WidgetInteractionComponent|SetVirtualUserIndex (Variables|Default|GetWidgetInteraction) (Math|Random|RandomInteger 99999)))