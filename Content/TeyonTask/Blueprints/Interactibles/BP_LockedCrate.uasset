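; BP_LockedCrate is an interactible crate actor that opens by destroying itself when a keycard is used on it.
; OnItemInteract casts the caller to the first-person character and accepts either "PrintedKeycard", whose durability it reduces through the inventory component, or "Keycard", which it leaves untouched.
; Both paths share a DoOnce before DestroyActor.
; An item pickup spawn tied to a MainQuest objective is present but unconnected, so it never runs.
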(event EventBeginPlay)

(event Collision|EventActorBeginOverlap
  (params (OtherActor :type Actor%20Object%20Reference)))

(event EventTick
  (params (DeltaSeconds :type Float%20%28single-precision%29)))

(event EventOnItemInteract
  (params (UsedItem :type Name :default "None") (EventCaller :type Actor%20Object%20Reference))
  (bind _asbp_teyon_first_person_character (Utilities|Casting|CastToBP_Teyon_FirstPersonCharacter EventCaller))
  (if (== UsedItem "PrintedKeycard")
    (Default|ReduceDurability (Variables|/Game/TeyonTask/Blueprints/PlayerCharacter/BP_Teyon_FirstPersonCharacter.BP_Teyon_FirstPersonCharacter_C|GetAC_InventoryComponent _asbp_teyon_first_person_character) 1e+02)
    (Utilities|FlowControl|DoOnce false :!label _label
      (:Completed
        (Actor|DestroyActor)))
    (elif (== UsedItem "Keycard")
      (goto _label))))

(fn ConstructionScript)