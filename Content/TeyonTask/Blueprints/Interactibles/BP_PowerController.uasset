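; BP_PowerController manages a group of powerboxes with a limit on how many may run at once.
; It binds to each box's toggle event, recounts running boxes and updates the power status widget's progress bar.
; Exceeding the limit deactivates the controller, sets every box destroyed, tints the widget and stops its animations.
; ChangePowerConnections, run at BeginPlay, either connects boxes and restores saved states or saves states and disconnects them, depending on IsActive.
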(event Custom|OnPowerboxToggle
  (bind _activeconnections (CallFunction|UpdateWidget))
  (CallFunction|DestroyConnections _activeconnections))

(event EventBeginPlay
  (Utilities|FlowControl|Sequence
    (:then_0
      (bind _asw_power_status (Utilities|Casting|CastToW_PowerStatus (UserInterface|GetWidget (Variables|Default|GetWidget))))
      (Variables|Default|SetPowerStatusWidgetRef _asw_power_status))
    (:then_1
      (for _array_element (Variables|Default|GetPowerConnectionArray)
        (EventDispatchers|BindEventtoEventToggled _array_element (delegate Custom|OnPowerboxToggle))))
    (:then_2
      (CallFunction|UpdateWidget))
    (:then_3
      (CallFunction|ChangePowerConnections))))

(event Collision|EventActorBeginOverlap
  (params (OtherActor :type Actor%20Object%20Reference)))

(event EventTick
  (params (DeltaSeconds :type Float%20%28single-precision%29)))

(event EventDestroyed
  (for _array_element (Variables|Default|GetPowerConnectionArray)
    (EventDispatchers|UnbindEventfromEventToggled _array_element (delegate Custom|OnPowerboxToggle))))

(fn ConstructionScript)

(fn UpdateWidget
  (bind _activecount (LocalVariables|GetActiveCount))
  (for _array_element (Variables|Default|GetPowerConnectionArray)
    (if (Variables|/Game/TeyonTask/Blueprints/Interactibles/BP_Powerbox.BP_Powerbox_C|GetIsRunning _array_element)
      (Math|Integer|IncrementInt (LocalVariables|GetActiveCount))))
  (Default|UpdateProgressBar (Variables|Default|GetPowerStatusWidgetRef) _activecount (Variables|Default|GetMaxActiveAtOnce))
  (return _activecount))

(fn DestroyConnections
  (params (ActiveCount :type Integer))
  (if (> ActiveCount (Variables|Default|GetMaxActiveAtOnce))
    (Utilities|FlowControl|Sequence
      (:then_0
        (Variables|Default|SetIsActive false))
      (:then_1
        (for _array_element (Variables|Default|GetPowerConnectionArray)
          (Default|ChangeDestroyState _array_element true)
          (Default|UpdateState _array_element)))
      (:then_2
        (Class|WidgetComponent|SetTintColorandOpacity (Variables|Default|GetWidget) "(R=0.000000,G=0.000000,B=0.000000,A=0.500000)"))
      (:then_3
        (Class|UserWidget|StopAllAnimations (Variables|Default|GetPowerStatusWidgetRef))))))

(fn ChangePowerConnections
  (if (Variables|Default|GetIsActive)
    (for _array_element (Variables|Default|GetPowerConnectionArray)
      (Variables|/Game/TeyonTask/Blueprints/Interactibles/BP_Powerbox.BP_Powerbox_C|SetPowerConnected _array_element true))
    (for _array_element_2 (Variables|Default|GetSavedRunning)
      (Default|AssignIsRunning _array_element_2 true))
    (for _array_element_3 (Variables|Default|GetSavedIdle)
      (Default|AssignIsRunning _array_element_3 false))
    (else
      (CallFunction|SavePreviousStates)
      (for _array_element_4 (Variables|Default|GetPowerConnectionArray)
        (Variables|/Game/TeyonTask/Blueprints/Interactibles/BP_Powerbox.BP_Powerbox_C|SetPowerConnected _array_element_4 false)
        (Default|AssignIsRunning _array_element_4 false)))))

(fn SavePreviousStates
  (Utilities|FlowControl|Sequence
    (:then_0
      (Utilities|Array|Clear (Variables|Default|GetSavedRunning))
      (Utilities|Array|Clear (Variables|Default|GetSavedIdle)))
    (:then_1
      (for _array_element (Variables|Default|GetPowerConnectionArray)
        (Utilities|Array|Add (select (Variables|/Game/TeyonTask/Blueprints/Interactibles/BP_Powerbox.BP_Powerbox_C|GetIsRunning _array_element) (Variables|Default|GetSavedRunning) (Variables|Default|GetSavedIdle)) _array_element)))))