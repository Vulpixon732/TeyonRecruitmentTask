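; BP_Machine is an interactible machine with three animated pistons and a light that shows whether it is active.
; AssignState sets IsActive and calls UpdateState, which swaps the light material and plays or stops the piston timeline that drives each piston's relative Z.
; The construction script also refreshes the light.
; ToggleActive only flips the flag without refreshing, and the experience, level and gold getters are stubs returning zero.
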(event Custom|ToggleAnimation
  (bind _pistonthree (Variables|Default|GetPistonThree))
  (bind _pistonone (Variables|Default|GetPistonOne))
  (bind _pistontwo (Variables|Default|GetPistonTwo))
  (bind _relativelocation (Variables|/Script/Engine.SceneComponent|GetRelativeLocation _pistonthree))
  (bind _relativelocation_2 (Variables|/Script/Engine.SceneComponent|GetRelativeLocation _pistonone))
  (bind _relativelocation_3 (Variables|/Script/Engine.SceneComponent|GetRelativeLocation _pistontwo))
  (if (Variables|Default|GetIsActive)
    (bind (_direction _pistonone_2 _pistontwo_2 _pistonthree_2) (Timeline|PistonAnimation Play)
      (:Update
        (Utilities|FlowControl|Sequence
          (:then_0
            (Transformation|SetRelativeLocation _pistonone (Math|Vector|MakeVector (.x _relativelocation_2) (.y _relativelocation_2) (.z _pistonone_2)) false true))
          (:then_1
            (Transformation|SetRelativeLocation _pistontwo (Math|Vector|MakeVector (.x _relativelocation_3) (.y _relativelocation_3) (.z _pistontwo_2)) false true))
          (:then_2
            (Transformation|SetRelativeLocation _pistonthree (Math|Vector|MakeVector (.x _relativelocation) (.y _relativelocation) (.z _pistonthree_2)) false true)))))
    (else
      (Timeline|PistonAnimation Stop))))

(event Custom|UpdateState
  (CallFunction|UpdateVisuals)
  (CallFunction|ToggleAnimation))

(event EventBeginPlay
  (Components|Timeline|SetPlayRate (Variables|Default|GetPistonAnimation) (Variables|Default|GetAnimationSpeed))
  (CallFunction|UpdateState))

(event Collision|EventActorBeginOverlap
  (params (OtherActor :type Actor%20Object%20Reference)))

(event EventTick
  (params (DeltaSeconds :type Float%20%28single-precision%29)))

(event EventAssignState
  (params (IsActive :type Boolean))
  (Variables|Default|SetIsActive IsActive)
  (CallFunction|UpdateState))

(fn ConstructionScript
  (CallFunction|UpdateVisuals))

(fn UpdateVisuals
  (Rendering|Material|SetMaterial (Variables|Default|GetLight) 0 (select (Variables|Default|GetIsActive) "/Engine/MapTemplates/Materials/BasicAsset03.BasicAsset03" "/Engine/MapTemplates/Materials/BasicAsset01.BasicAsset01")))

(fn GetNeededExperience
  (return 0.0))

(fn GetCharacterLevel
  (return 0))

(fn GetExperience
  (return 0.0))

(fn GetGold
  (return 0))

(fn ToggleActive
  (Variables|Default|SetIsActive (not (Variables|Default|GetIsActive))))