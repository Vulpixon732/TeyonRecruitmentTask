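; BP_MainDoor is an interactable double sliding door that a keypad toggles or a crowbar forces open.
; OnInteract only accepts a BP_Keypad caller, and ToggleDoor uses a FlipFlop to play or reverse a timeline that slides both leaves apart along Y.
; Crowbar use on an active door not marked open reduces durability through the player's inventory component, toggles the door, then deactivates it.
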(event Custom|ToggleDoor
  (bind _openingdistance (Variables|Default|GetOpeningDistance))
  (if (Variables|Default|GetIsActive)
    (bind _isa (Utilities|FlowControl|FlipFlop)
      (:A
        (bind _lerp (Timeline|DoorAnimationTimeline Play)
          (:Update
            (Utilities|FlowControl|Sequence
              (:then_0
                (Transformation|SetRelativeLocation (Variables|Default|GetDoorLeft) (Math|Vector|MakeVector 0.0 (Math|Float|Lerp 0.0 (* _openingdistance -1.0) _lerp) 0.0) false true))
              (:then_1
                (Transformation|SetRelativeLocation (Variables|Default|GetDoorRight) (Math|Vector|MakeVector 0.0 (Math|Float|Lerp 0.0 _openingdistance _lerp) 0.0) false true))))
          (:Finished
            (Variables|Default|SetIsOpen _isa))))
      (:B
        (Timeline|DoorAnimationTimeline Reverse)))))

(event EventBeginPlay)

(event Collision|EventActorBeginOverlap
  (params (OtherActor :type Actor%20Object%20Reference)))

(event EventTick
  (params (DeltaSeconds :type Float%20%28single-precision%29)))

(event EventOnInteract
  (params (PlayerActor :type Actor%20Object%20Reference))
  (Utilities|Casting|CastToBP_Keypad PlayerActor)
  (CallFunction|ToggleDoor))

(event EventOnItemInteract
  (params (UsedItem :type Name :default "None") (EventCaller :type Actor%20Object%20Reference))
  (bind _asbp_teyon_first_person_character (Utilities|Casting|CastToBP_Teyon_FirstPersonCharacter EventCaller))
  (if (Math|Boolean|ANDBoolean (== UsedItem "Crowbar") (not (Variables|Default|GetIsOpen)) (Variables|Default|GetIsActive))
    (Default|ReduceDurability (Variables|/Game/TeyonTask/Blueprints/PlayerCharacter/BP_Teyon_FirstPersonCharacter.BP_Teyon_FirstPersonCharacter_C|GetAC_InventoryComponent _asbp_teyon_first_person_character) 1e+02)
    (CallFunction|ToggleDoor)
    (Variables|Default|SetIsActive false)))

(fn ConstructionScript)