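; Electric gate interactible that switches a barrier on or off through the IsActive flag.
; UpdateEntranceState toggles visibility and collision (QueryAndProbe or none) on a set of cube components and an InvisibleWall.
; It runs from the Construction Script, BeginPlay and a Debug_Update event.
; SetActive only stores the flag and does not refresh the components itself.
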(event Custom|Debug_Update
  (CallFunction|UpdateEntranceState))

(event EventBeginPlay
  (CallFunction|UpdateEntranceState))

(event Collision|EventActorBeginOverlap
  (params (OtherActor :type Actor%20Object%20Reference)))

(event EventTick
  (params (DeltaSeconds :type Float%20%28single-precision%29)))

(fn ConstructionScript
  (CallFunction|UpdateEntranceState))

(fn SetActive
  (params (IsActive :type Boolean))
  (Variables|Default|SetIsActive IsActive))

(fn UpdateEntranceState
  (bind _isactive (Variables|Default|GetIsActive))
  (for _array_element (Utilities|Array|MakeArray (Variables|Default|GetCube11) (Variables|Default|GetInvisibleWall) (Variables|Default|GetCube10) (Variables|Default|GetCube9) (Variables|Default|GetCube8) (Variables|Default|GetCube7) (Variables|Default|GetCube6) (Variables|Default|GetCube5) (Variables|Default|GetCube4) (Variables|Default|GetCube3))
    (Rendering|SetVisibility _array_element _isactive false)
    (Collision|SetCollisionEnabled _array_element (select _isactive "QueryAndProbe" "NoCollision"))))