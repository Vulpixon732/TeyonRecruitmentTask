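; Player inventory component holding up to three items in an array, mirrored to hotbar widgets that are rebuilt as items change.
; Keys 1–3 select the active slot, and Q drops that item as a BP_ItemPickup carrying its quest IDs and durability.
; Newly added quests get objective credit for matching items already held.
; Durability loss destroys depleted items, aborting the quest linked to a destroyed item.
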(event Custom|OnQuestAdded
  (params (QuestID :type Name) (QuestInfo :type ST%20Quest%20Info%20Structure) (MultipleQuestsAdded? :type Boolean))
  (for _array_element (Variables|Default|GetItemDataArray)
    (if (== (.questid _array_element) QuestID)
      (Default|AddObjectiveAmount (Variables|/Game/TeyonTask/Blueprints/PlayerCharacter/BP_Teyon_FirstPersonCharacter.BP_Teyon_FirstPersonCharacter_C|GetBP_BPC_PlayerQuestComponent (stale EventBeginPlay _asbp_teyon_first_person_character)) (.questid _array_element) (.objectiveid _array_element) 1))))

(event EventBeginPlay
  (bind _asbp_teyon_first_person_character (Utilities|Casting|CastToBP_Teyon_FirstPersonCharacter (Game|GetPlayerCharacter 0)))
  (EventDispatchers|BindEventtoOnQuestAdded (Variables|/Game/TeyonTask/Blueprints/PlayerCharacter/BP_Teyon_FirstPersonCharacter.BP_Teyon_FirstPersonCharacter_C|GetBP_BPC_PlayerQuestComponent _asbp_teyon_first_person_character) (delegate Custom|OnQuestAdded)))

(event EventTick
  (params (DeltaSeconds :type Float%20%28single-precision%29)))

(event Input|KeyboardEvents|1
  (params (Key :type Key%20Structure :default "None"))
  (:Pressed
    (CallFunction|SetActiveSlot)))

(event Input|KeyboardEvents|2
  (params (Key :type Key%20Structure :default "None"))
  (:Pressed
    (CallFunction|SetActiveSlot 1)))

(event Input|KeyboardEvents|3
  (params (Key :type Key%20Structure :default "None"))
  (:Pressed
    (CallFunction|SetActiveSlot 2)))

(event Input|KeyboardEvents|Q
  (params (Key :type Key%20Structure :default "None"))
  (:Pressed
    (CallFunction|DropItem)))

(fn SetActiveSlot
  (params (TargetSlot :type Integer))
  (Variables|Default|SetActiveSlot TargetSlot)
  (Default|UpdateBorderColor (Variables|Default|GetInventoryHotbarRef) TargetSlot))

(fn AddtoInventory
  (params (ItemStruct :type S%20Item%20Data%20Structure))
  (if (<= (Utilities|Array|Length (Variables|Default|GetItemDataArray)) 2)
    (Utilities|Array|Add (Variables|Default|GetItemDataArray) ItemStruct)
    (CallFunction|RefreshHotbar)
    (return true)
    (else
      (Development|PrintString "Not enough inventory space")
      (return false))))

(fn RefreshHotbar
  (bind _inventoryhotbarref (Variables|Default|GetInventoryHotbarRef))
  (bind _inventoryhotbarref_2 (Variables|Default|GetInventoryHotbarRef))
  (Utilities|FlowControl|Sequence
    (:then_0
      (Utilities|FlowControl|Sequence
        (:then_0
          (Widget|Panel|ClearChildren (Variables|/Game/TeyonTask/Blueprints/Widgets/Inventory/W_InventoryHotbar.W_InventoryHotbar_C|GetSlot1 _inventoryhotbarref_2)))
        (:then_1
          (Widget|Panel|ClearChildren (Variables|/Game/TeyonTask/Blueprints/Widgets/Inventory/W_InventoryHotbar.W_InventoryHotbar_C|GetSlot2 _inventoryhotbarref_2)))
        (:then_2
          (Widget|Panel|ClearChildren (Variables|/Game/TeyonTask/Blueprints/Widgets/Inventory/W_InventoryHotbar.W_InventoryHotbar_C|GetSlot3 _inventoryhotbarref_2)))))
    (:then_1
      (for (_array_element _array_index) (Variables|Default|GetItemDataArray)
        (bind _returnvalue (UserInterface|CreateWidget "/Game/TeyonTask/Blueprints/Widgets/Inventory/W_ItemIcon.W_ItemIcon_C" 0 (.Name (Utilities|Struct|BreakS_ItemData _array_element)) (.Durability (Utilities|Struct|BreakS_ItemData _array_element))))
        (Widget|Panel|AddChild (Utilities|Select :Index _array_index :Option%200 (Variables|/Game/TeyonTask/Blueprints/Widgets/Inventory/W_InventoryHotbar.W_InventoryHotbar_C|GetSlot1 _inventoryhotbarref) :Option%201 (Variables|/Game/TeyonTask/Blueprints/Widgets/Inventory/W_InventoryHotbar.W_InventoryHotbar_C|GetSlot2 _inventoryhotbarref) :Option%202 (Variables|/Game/TeyonTask/Blueprints/Widgets/Inventory/W_InventoryHotbar.W_InventoryHotbar_C|GetSlot3 _inventoryhotbarref)) _returnvalue)))))

(fn DropItem
  (params (OverrideTransform :type Boolean) (TargetTransform :type Transform) (DurabilityPenalty :type Float%20%28double-precision%29))
  (bind _itemdataarray (Variables|Default|GetItemDataArray))
  (bind _activeslot (Variables|Default|GetActiveSlot))
  (bind _output (Utilities|Array|Get(acopy) _itemdataarray _activeslot))
  (bind (_name _questid _objectiveid _durability) (Utilities|Struct|BreakS_ItemData _output))
  (if (Utilities|Array|IsValidIndex (Variables|Default|GetItemDataArray) (Variables|Default|GetActiveSlot))
    (bind _returnvalue (Game|SpawnActorfromClass "/Game/TeyonTask/Blueprints/Items/BP_ItemPickup.BP_ItemPickup_C" (Math|Transform|SelectTransform TargetTransform (Transformation|GetActorTransform (Game|GetPlayerCharacter 0)) OverrideTransform) "AdjustIfPossibleButAlwaysSpawn" "MultiplyWithRoot" 0 (Utilities|Struct|MakeS_ItemData _name _questid _objectiveid (- _durability DurabilityPenalty)) _questid _objectiveid 0))
    (Utilities|IsValid _returnvalue
      (:Is%20Valid
        (Default|DropfromInventory _returnvalue)
        (Default|CheckDurability _returnvalue)
        (Utilities|Array|RemoveIndex (Variables|Default|GetItemDataArray) (Variables|Default|GetActiveSlot))
        (CallFunction|RefreshHotbar)))))

(fn FetchActiveItemData
  (return (Utilities|Array|Get(acopy) (Variables|Default|GetItemDataArray) (Variables|Default|GetActiveSlot))))

(fn DestroyActiveItem
  (bind _itemdataarray (Variables|Default|GetItemDataArray))
  (bind _activeslot (Variables|Default|GetActiveSlot))
  (bind _output (Utilities|Array|Get(acopy) _itemdataarray _activeslot))
  (Utilities|FlowControl|Sequence
    (:then_0
      (if (!= (.questid _output) "None")
        (bind _asbp_teyon_first_person_character (Utilities|Casting|CastToBP_Teyon_FirstPersonCharacter (Game|GetPlayerCharacter 0)))
        (Default|OnQuestAbortedEvent (Variables|/Game/TeyonTask/Blueprints/PlayerCharacter/BP_Teyon_FirstPersonCharacter.BP_Teyon_FirstPersonCharacter_C|GetBP_BPC_PlayerQuestComponent _asbp_teyon_first_person_character) (.questid _output) (Default|GetQuestInfo (Variables|/Game/TeyonTask/Blueprints/PlayerCharacter/BP_Teyon_FirstPersonCharacter.BP_Teyon_FirstPersonCharacter_C|GetBP_BPC_PlayerQuestComponent _asbp_teyon_first_person_character) (.questid _output)))))
    (:then_1
      (Utilities|Array|RemoveIndex (Variables|Default|GetItemDataArray) (Variables|Default|GetActiveSlot))
      (CallFunction|RefreshHotbar))))

(fn ReduceDurability
  (params (Penalty :type Float%20%28double-precision%29))
  (bind _activeslot (Variables|Default|GetActiveSlot))
  (bind _itemdataarray (Variables|Default|GetItemDataArray))
  (bind _output (Utilities|Array|Get(acopy) _itemdataarray _activeslot))
  (Utilities|Array|SetArrayElem (Variables|Default|GetItemDataArray) (Variables|Default|GetActiveSlot) (Utilities|Struct|MakeS_ItemData (.name _output) (.questid _output) (.objectiveid _output) (- (.durability _output) Penalty)))
  (if (<= (.durability (CallFunction|FetchActiveItemData)) 0.0)
    (CallFunction|DestroyActiveItem)
    (else
      (CallFunction|RefreshHotbar))))