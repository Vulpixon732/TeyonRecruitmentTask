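; BP_ThrowImpactPreview is a preview actor that, judging by its name, marks where a thrown item will land.
; On BeginPlay, the ThrobbingAnimation timeline pulses the Cylinder's X and Y scale while keeping its Z scale.
; UpdateTrace moves the Start component to a given location when it changes, then sets the Niagara beam's endpoints from the Start and Target world positions.
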(event Custom|UpdateTrace
  (params (NewLocation :type Vector))
  (bind _niagara (Variables|Default|GetNiagara))
  (bind _start (Variables|Default|GetStart))
  (if (Utilities|Operators|NotEqual(!=) (Transformation|GetWorldLocation _start) NewLocation 0.0)
    (Transformation|SetWorldLocation _start NewLocation false true)
    (Niagara|SetNiagaraVariable(Vector3) _niagara "Beam Start" (Transformation|GetWorldLocation (Variables|Default|GetStart)))
    (Niagara|SetNiagaraVariable(Vector3) _niagara "Beam End" (Transformation|GetWorldLocation (Variables|Default|GetTarget)))))

(event EventBeginPlay
  (bind _scale (Timeline|ThrobbingAnimation Play)
    (:Update
      (Transformation|SetRelativeScale3D (Variables|Default|GetCylinder) (Math|Vector|MakeVector _scale _scale (.z (Variables|/Script/Engine.SceneComponent|GetRelativeScale3D (Variables|Default|GetCylinder))))))))

(event Collision|EventActorBeginOverlap
  (params (OtherActor :type Actor%20Object%20Reference)))

(event EventTick
  (params (DeltaSeconds :type Float%20%28single-precision%29)))

(fn ConstructionScript)