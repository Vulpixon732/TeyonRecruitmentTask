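; Interactable item pickup that goes into the player's inventory and keeps quest objective progress in sync when dropped.
; On BeginPlay it copies its quest and objective IDs into its item struct.
; Interacting adds that struct to the first-person character's inventory component, and only on success runs the parent interaction and destroys the actor.
; Dropping it from inventory decrements the linked objective through the quest component when both IDs are set.
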(event Custom|DropFromInventory
  (if (and (!= (Variables|Default|GetQuestID) "None") (!= (Variables|Default|GetObjectiveID) "None"))
    (Default|AddObjectiveAmount (Variables|Default|GetQuestComponent) (Variables|Default|GetQuestID) (Variables|Default|GetObjectiveID) -1)))

(event EventBeginPlay
  (|CallParentFunction)
  (Variables|Default|SetItem_Struct (Utilities|Struct|MakeS_ItemData (.name (Variables|Default|GetItem_Struct)) (.actorreference (Variables|Default|GetItem_Struct)) (Variables|Default|GetQuestID) (Variables|Default|GetObjectiveID))))

(event Collision|EventActorBeginOverlap
  (params (OtherActor :type Actor%20Object%20Reference)))

(event EventTick
  (params (DeltaSeconds :type Float%20%28single-precision%29)))

(event EventOnInteract
  (params (PlayerActor :type Actor%20Object%20Reference))
  (bind _itemadded (CallFunction|AddtoInventory))
  (if _itemadded
    (|CallParentFunction 0)
    (Utilities|IsValid self
      (:Is%20Valid
        (Actor|DestroyActor)))))

(fn ConstructionScript
  (|CallParentFunction))

(fn AddtoInventory
  (bind _asbp_teyon_first_person_character (Utilities|Casting|CastToBP_Teyon_FirstPersonCharacter (Game|GetPlayerCharacter 0)))
  (bind _itemadded (Default|AddtoInventory (Variables|/Game/TeyonTask/Blueprints/PlayerCharacter/BP_Teyon_FirstPersonCharacter.BP_Teyon_FirstPersonCharacter_C|GetAC_InventoryComponent _asbp_teyon_first_person_character) (Variables|Default|GetItem_Struct)))
  (return _itemadded))